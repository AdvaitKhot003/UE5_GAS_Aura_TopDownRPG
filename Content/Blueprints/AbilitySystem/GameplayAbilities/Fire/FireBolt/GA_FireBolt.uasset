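; GA_FireBolt is the fire bolt gameplay ability, which casts a projectile at the point under the mouse.
; On activation it gets target data under the cursor and turns the avatar toward that location through CombatInterface.
; It plays the cast montage and spawns the projectile when the montage's FireBolt gameplay event arrives.
; The ability ends when the montage completes, blends out, is interrupted or is cancelled.
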(event Ability|EventActivateAbility
  (bind _targetdatahandle (|TargetDataUnderMouse)
    (:ValidTargetData
      (Variables|Default|SetTarget%20Location (.Location (Collision|BreakHitResult (Ability|TargetData|GetHitResultfromTargetData _targetdatahandle))))
      (bind _ascombat_interface (Utilities|Casting|CastToCombatInterface (Ability|GetAvatarActorfromActorInfo)))
      (Class|CombatInterface|UpdateFacingDirection _ascombat_interface (Variables|Default|GetTarget%20Location))
      (|PlayMontageandWaitProxy "None" "/Game/Blueprints/Character/Aura/Montages/AM_Cast_FireBolt.AM_Cast_FireBolt" 1.0 "None" true 1.0 0.0 false
        (:then
          (Ability|Tasks|WaitGameplayEvent "(TagName=\"EventTag.Montage.FireBolt\")" 0
            (:EventReceived
              (Class|AuraProjectileSpellAbility|SpawnProjectile (Variables|Default|GetTarget%20Location)))))
        (:OnCompleted
          (Ability|EndAbility :!label _label))
        (:OnBlendOut
          (goto _label))
        (:OnInterrupted
          (goto _label))
        (:OnCancelled
          (goto _label))))))

(event Ability|EventOnEndAbility
  (params (bWasCancelled :type Boolean)))